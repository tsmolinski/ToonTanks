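; Player controller for the frontend that brings up the main menu when play begins.
; On BeginPlay it creates a BP_UI_Base widget, adds it to the viewport, pushes BP_UI_MainMenu onto it and shows the mouse cursor.
; It keeps a reference to that base widget and forwards PushPrompt calls, with their text, owner and index, to it.
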(event Custom|ActivateMainMenu
  (bind _returnvalue (UserInterface|CreateWidget "/Game/UI/BP_UI_Base.BP_UI_Base_C" self))
  (Variables|Default|SetBP_UI_Base _returnvalue)
  (UserInterface|Viewport|AddtoViewport _returnvalue 0)
  (Default|PushMenu _returnvalue "/Game/UI/BP_UI_MainMenu.BP_UI_MainMenu_C")
  (Variables|/Script/Engine.PlayerController|SetbShowMouseCursor (Game|GetPlayerController 0) true))

(event Custom|PushPrompt
  (params (InPromptText :type Text) (InPromptOwner :type BP%20UI%20Main%20Menu%20Object%20Reference) (InPromptIndex :type Integer))
  (Default|PushPrompt (Variables|Default|GetBP_UI_Base) InPromptText InPromptOwner InPromptIndex))

(event EventBeginPlay
  (CallFunction|ActivateMainMenu))

(fn ConstructionScript)